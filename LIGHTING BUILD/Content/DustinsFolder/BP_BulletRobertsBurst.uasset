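; BP_BulletRobertsBurst is a bullet projectile actor that bursts on its first hit and otherwise expires three seconds after spawning.
; A one-shot Hit handler adds a Niagara effect offset above the mesh and plays a quiet impact sound.
; It then hides the mesh and its existing Niagara component, destroying the actor a second later.
; Despite the graph's comment, the hit logic applies no physics impulse.
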(event Collision|EventHit
  (params (MyComp :type Primitive%20Component%20Object%20Reference) (Other :type Actor%20Object%20Reference) (OtherComp :type Primitive%20Component%20Object%20Reference) (bSelfMoved :type Boolean) (HitLocation :type Vector :default "0, 0, 0") (HitNormal :type Vector :default "0, 0, 0") (NormalImpulse :type Vector :default "0, 0, 0") (Hit :type Hit%20Result%20Structure%20%28by%20ref%29))
  (bind _staticmesh (Variables|Default|GetStaticMesh))
  (bind _returnvalue (Transformation|GetWorldLocation _staticmesh))
  ;[1 1 1] physics impluse to hit object
  (Utilities|FlowControl|DoOnce false
    (:Completed
      (Variables|Default|SetHitLoc (Transformation|GetActorLocation))
      (bind _output_get (Variables|Default|SetHitTraqns (Transformation|GetActorTransform)))
      (AddComponent|AddNiagaraComponent true (Math|Transform|MakeTransform (Math|Vector|MakeVector (.x _returnvalue) (.y _returnvalue) (+ (.z _returnvalue) 5e+01)) (.rotation _output_get) (.scale _output_get)))
      (Audio|SpawnSoundatLocation "/Game/RobertFunZone/Audio/BallHitNew.BallHitNew" (Transformation|GetWorldLocation (Variables|Default|GetStaticMesh)) "0, 0, 0" 0.05 1.0 0.0 0 0)
      (Rendering|SetVisibility (Variables|Default|GetStaticMesh) false false)
      (Utilities|FlowControl|Delay 1.0)
      (Actor|DestroyActor))))

(event EventBeginPlay
  ;[1 1 1] Destroys bullet after 3 seconds of airtime
  (Utilities|FlowControl|Delay 3.0)
  (Actor|DestroyActor))

(fn ConstructionScript)