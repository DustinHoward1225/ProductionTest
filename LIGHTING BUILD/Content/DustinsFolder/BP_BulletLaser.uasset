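; Laser bullet projectile actor that removes itself after a short lifetime or shortly after it hits something.
; On its first hit, it spawns a separate death-effect actor at the Niagara component's transform and plays an impact sound there.
; It then hides its particle, light and Niagara components, waits briefly, and destroys both the effect actor and itself.
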(event Custom|hit
  (bind _niagara (Variables|Default|GetNiagara))
  ;[1 1 1] Once the bullet hits something, it would spawn the death effect, play the sound, then hides everything else and deletes the actor a second after.
  (Utilities|FlowControl|DoOnce false
    (:Completed
      (Variables|Default|SetHit%20Loc (Transformation|GetActorLocation))
      (bind _output_get (Variables|Default|SetHit%20Traqns (Transformation|GetWorldTransform _niagara)))
      (bind _returnvalue (Game|SpawnActorfromClass "/Game/DustinsFolder/particles/LaserDeathEffectBP.LaserDeathEffectBP_C" (Math|Transform|MakeTransform (.location _output_get) (.rotation _output_get) "1,1,1") "Undefined" 0 0))
      (Audio|SpawnSoundatLocation "/Game/RobertFunZone/Audio/LaserHit.LaserHit" (Transformation|GetWorldLocation _niagara) "0, 0, 0" 0.05 1.0 0.0 0 0)
      (Rendering|SetVisibility (Variables|Default|GetParticleSystem) false false)
      (Utilities|FlowControl|Delay 1.0)
      (Actor|DestroyActor _returnvalue)
      (Actor|DestroyActor))))

(event Collision|EventHit
  (params (MyComp :type Primitive%20Component%20Object%20Reference) (Other :type Actor%20Object%20Reference) (OtherComp :type Primitive%20Component%20Object%20Reference) (bSelfMoved :type Boolean) (HitLocation :type Vector :default "0, 0, 0") (HitNormal :type Vector :default "0, 0, 0") (NormalImpulse :type Vector :default "0, 0, 0") (Hit :type Hit%20Result%20Structure%20%28by%20ref%29))
  ;[1 1 1] Once the bullet hits something, it would spawn the death effect, play the sound, then hides everything else and deletes the actor a second after.
  (CallFunction|Hit))

(event EventBeginPlay
  ;[1 1 1] After 3 seconds destroys bullet
  (Utilities|FlowControl|Delay 3.0)
  (Actor|DestroyActor))

(fn ConstructionScript)