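; BP_BulletMagnet is a short-lived homing projectile that destroys itself five seconds after spawning.
; An overlap on component R with a VeryPlaceholderGun steers its ProjectileMovement toward that actor's mesh with strong homing acceleration.
; CHase2 applies the same homing to a supplied target's mesh, while Chase homes on a static mesh component it newly adds to its target.
; A loop over all VeryPlaceholderGun actors is left unconnected.
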(event OnComponentBeginOverlap(r)
  (params (OverlappedComponent :type Primitive%20Component%20Object%20Reference) (OtherActor :type Actor%20Object%20Reference) (OtherComp :type Primitive%20Component%20Object%20Reference) (OtherBodyIndex :type Integer) (bFromSweep :type Boolean) (SweepResult :type Hit%20Result%20Structure%20%28by%20ref%29))
  (bind _projectilemovement (Variables|Default|GetProjectileMovement))
  (bind _asvery_placeholder_gun (Utilities|Casting|CastToVeryPlaceholderGun OtherActor))
  (Variables|/Script/Engine.ProjectileMovementComponent|SetHomingTargetComponent _projectilemovement (Variables|/Game/RobertFunZone/Gun/VeryPlaceholderGun.VeryPlaceholderGun_C|GetStaticMesh _asvery_placeholder_gun))
  (Variables|/Script/Engine.ProjectileMovementComponent|SetHomingAccelerationMagnitude _projectilemovement 2.5e+04))

(event Custom|Chase
  (params (Target :type Actor%20Object%20Reference))
  (bind _returnvalue (AddComponent|AddStaticMeshComponent Target false))
  (if (Utilities|IsValid _returnvalue)
    (Variables|/Script/Engine.ProjectileMovementComponent|SetHomingTargetComponent (Variables|Default|GetProjectileMovement) _returnvalue)))

(event Custom|CHase2
  (params (Targettohit :type Static%20Mesh%20Actor%20Object%20Reference))
  (bind _projectilemovement (Variables|Default|GetProjectileMovement))
  (if (Utilities|IsValid Targettohit)
    (Variables|/Script/Engine.ProjectileMovementComponent|SetHomingTargetComponent _projectilemovement (Variables|/Script/Engine.StaticMeshActor|GetStaticMeshComponent Targettohit))
    (Variables|/Script/Engine.ProjectileMovementComponent|SetHomingAccelerationMagnitude _projectilemovement 2.5e+04)))

(event Collision|EventActorBeginOverlap
  (params (OtherActor :type Actor%20Object%20Reference)))

(event EventTick
  (params (DeltaSeconds :type Float%20%28single-precision%29)))

(event EventBeginPlay
  (Utilities|FlowControl|Delay 5.0)
  (Actor|DestroyActor))

(fn ConstructionScript)