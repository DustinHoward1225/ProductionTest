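; VR spear actor that can be picked up, dropped, rotated, and used to skewer and fling objects.
; Overlaps on its end box record an Engine or VeryPlaceholderGun enemy and attach the Engine's root to the spear.
; At BeginPlay it binds to MotionControllerPawn dispatchers: tip-off enables physics and applies an impulse to the skewered meshes, while rotate drives a roll timeline from the Stick value.
; Pickup and Drop toggle physics and attachment; Tick prints Stick for debugging.
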(event OnComponentBeginOverlap(EndBox)
  (params (OverlappedComponent :type Primitive%20Component%20Object%20Reference) (OtherActor :type Actor%20Object%20Reference) (OtherComp :type Primitive%20Component%20Object%20Reference) (OtherBodyIndex :type Integer) (bFromSweep :type Boolean) (SweepResult :type Hit%20Result%20Structure%20%28by%20ref%29))
  (bind _asvery_placeholder_gun (Utilities|Casting|CastToVeryPlaceholderGun OtherActor)
    (:then
      (Variables|Default|SetEngine? false)
      (bind _output_get (Variables|Default|SetEnemyStabbed _asvery_placeholder_gun)))
    (:CastFailed
      (bind _asengine (Utilities|Casting|CastToEngine OtherActor))
      (Variables|Default|SetEngine? true)
      (bind _output_get_2 (Variables|Default|SetEngine _asengine))))
  (Transformation|AttachComponentToComponent (Variables|/Script/Engine.Actor|GetRootComponent _output_get_2) (Variables|Default|Getw) "None" "KeepRelative" "KeepRelative" "KeepWorld" true))

(event Custom|RotateSpear_Event_0
  (Math|Float|CompareFloat (Variables|Default|Getstick) 0.0
    (:>
      (bind _newtrack_0 (Timeline|RotateSpear Play)
        (:Update
          (Transformation|SetActorRelativeRotation (Math|Rotator|MakeRotator (Math|Float|Lerp (.roll (Transformation|GetActorRotation)) _newtrack_0 0.4) 0.0 0.0)))))
    (:==
      (Timeline|RotateSpear Stop))
    (:<
      (Timeline|RotateSpear Reverse))))

(event Custom|TipoffSpear_Event_0
  (bind _engine (Variables|Default|GetEngine))
  (bind _enemystabbed (Variables|Default|GetEnemyStabbed))
  (bind _staticmesh (Variables|/Game/RobertFunZone/Gun/VeryPlaceholderGun.VeryPlaceholderGun_C|GetStaticMesh _enemystabbed))
  (bind _sphere (Variables|/Game/Engine.Engine_C|GetSphere _engine))
  (Physics|SetSimulatePhysics _sphere true)
  (if (Variables|Default|GetEngine?)
    (Physics|AddImpulseatLocation _sphere "5000.000000,5000.000000,5000.000000" (Variables|/Script/Engine.SceneComponent|GetRelativeLocation _sphere) "None")
    (else
      (Physics|AddImpulseatLocation _staticmesh "5000.000000,5000.000000,5000.000000" (Variables|/Script/Engine.SceneComponent|GetRelativeLocation _staticmesh) "None"))))

(event EventBeginPlay
  (bind _outactors (Actor|GetAllActorsOfClass "/Game/VirtualRealityBP/Blueprints/MotionControllerPawn.MotionControllerPawn_C"))
  (bind _array_element (Utilities|Array|ForEachLoopwithBreak _outactors)
    (:LoopBody
      (bind _asmotion_controller_pawn (Utilities|Casting|CastToMotionControllerPawn _array_element))
      (EventDispatchers|AssignRotateSpear _asmotion_controller_pawn (delegate Custom|RotateSpear_Event_0))
      (EventDispatchers|AssignTipoffSpear _asmotion_controller_pawn (delegate Custom|TipoffSpear_Event_0)))))

(event EventTick
  (params (DeltaSeconds :type Float%20%28single-precision%29))
  (Development|PrintString (Utilities|String|ToString(Float) (Variables|Default|Getstick))))

(event EventDrop
  (Physics|SetSimulatePhysics (Variables|Default|GetCylinder) true)
  (Transformation|DetachFromActor "KeepWorld" "KeepWorld" "KeepWorld"))

(event EventPickup
  (params (AttachTo :type Scene%20Component%20Object%20Reference))
  (Physics|SetSimulatePhysics (Variables|Default|GetCylinder) false)
  (Transformation|AttachComponentToComponent (VehicleSound|GetRootComponent) AttachTo "None" "KeepWorld" "KeepWorld" "KeepWorld" true))

(fn ConstructionScript)