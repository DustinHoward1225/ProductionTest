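; BP_BulletLandmine is a projectile landmine that travels until a MotionControllerPawn's LandMine1Press event detonates it.
; While Moving, Tick plays the Travel timeline, lerping toward its forward vector times a fixed distance, a world position rather than an offset.
; Detonation stops movement, shows BIGBOOM, enables Box collision to destroy overlapping VeryPlaceholderGun actors, then self-destructs after a delay.
; BeginPlay also draws a persistent debug trace forward, whose result is unused.
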(event OnComponentBeginOverlap(Box)
  (params (OverlappedComponent :type Primitive%20Component%20Object%20Reference) (OtherActor :type Actor%20Object%20Reference) (OtherComp :type Primitive%20Component%20Object%20Reference) (OtherBodyIndex :type Integer) (bFromSweep :type Boolean) (SweepResult :type Hit%20Result%20Structure%20%28by%20ref%29))
  (bind _asvery_placeholder_gun (Utilities|Casting|CastToVeryPlaceholderGun OtherActor))
  (Actor|DestroyActor _asvery_placeholder_gun))

(event Custom|LandMine1Press_Event_0
  (Variables|Default|SetMoving false)
  (Rendering|SetVisibility (Variables|Default|GetBIGBOOM) true false)
  (Collision|SetCollisionEnabled (Variables|Default|GetBox) "QueryAndPhysics")
  (Utilities|FlowControl|Delay 2.0)
  (Actor|DestroyActor))

(event Collision|EventActorBeginOverlap
  (params (OtherActor :type Actor%20Object%20Reference)))

(event EventTick
  (params (DeltaSeconds :type Float%20%28single-precision%29))
  (bind _outactors (Actor|GetAllActorsOfClass "/Game/VirtualRealityBP/Blueprints/MotionControllerPawn.MotionControllerPawn_C"))
  (bind _array_element (Utilities|Array|ForEachLoopwithBreak _outactors)
    (:LoopBody
      (if (Variables|Default|GetMoving)
        (bind _newtrack_0 (Timeline|Travel Play)
          (:Update
            (Transformation|SetWorldLocation (Variables|Default|GetDefaultSceneRoot) (Math|Vector|Lerp(Vector) (Transformation|GetActorLocation) (* (Transformation|GetActorForwardVector) 2e+03) _newtrack_0) false false)))
        (else
          (Timeline|Travel Stop))))))

(event EventBeginPlay
  (bind _returnvalue (Transformation|GetActorLocation))
  (Rendering|SetVisibility (Variables|Default|GetBIGBOOM) false false)
  (Collision|SetCollisionEnabled (Variables|Default|GetBox) "NoCollision")
  (bind _outactors (Actor|GetAllActorsOfClass "/Game/VirtualRealityBP/Blueprints/MotionControllerPawn.MotionControllerPawn_C"))
  (bind _array_element (Utilities|Array|ForEachLoopwithBreak _outactors)
    (:LoopBody
      (EventDispatchers|AssignLandMine1Press _array_element (delegate Custom|LandMine1Press_Event_0))
      (Collision|LineTraceByChannel _returnvalue (+ _returnvalue (* (Transformation|GetActorForwardVector) 2e+05)) "TraceTypeQuery1" false 0 "Persistent"))))

(fn ConstructionScript)