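; Homing bullet that seeks the nearest VeryPlaceholderGun actor.
; On BeginPlay, MoveToTarget calls FindTarget once and sets the result as the ProjectileMovement homing target.
; FindTarget loops over every VeryPlaceholderGun, compares mesh distance to the bullet against ClosestDistance, and returns the closest one's StaticMesh.
; Chase, CHase2 and overlap events are empty, and several disconnected leftover experiments never run.
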(event OnComponentBeginOverlap(r)
  (params (OverlappedComponent :type Primitive%20Component%20Object%20Reference) (OtherActor :type Actor%20Object%20Reference) (OtherComp :type Primitive%20Component%20Object%20Reference) (OtherBodyIndex :type Integer) (bFromSweep :type Boolean) (SweepResult :type Hit%20Result%20Structure%20%28by%20ref%29)))

(event Custom|Chase
  (params (Target :type Actor%20Object%20Reference)))

(event Custom|CHase2
  (params (Targettohit :type Static%20Mesh%20Actor%20Object%20Reference)))

(event Custom|MoveToTarget
  (bind _closest (CallFunction|FindTarget))
  (Variables|/Script/Engine.ProjectileMovementComponent|SetHomingTargetComponent (Variables|Default|GetProjectileMovement) _closest))

(event Collision|EventActorBeginOverlap
  (params (OtherActor :type Actor%20Object%20Reference)))

(event EventTick
  (params (DeltaSeconds :type Float%20%28single-precision%29)))

(event EventBeginPlay
  (CallFunction|MovetoTarget))

(fn ConstructionScript)

(fn FindTarget
  (bind _outactors (Actor|GetAllActorsOfClass "/Game/RobertFunZone/Gun/VeryPlaceholderGun.VeryPlaceholderGun_C"))
  (for _array_element _outactors
    (if (< (Math|Vector|VectorLength (- (Transformation|GetWorldLocation (Variables|/Game/RobertFunZone/Gun/VeryPlaceholderGun.VeryPlaceholderGun_C|GetStaticMesh _array_element)) (Transformation|GetActorLocation))) (LocalVariables|GetClosestDistance))
      (LocalVariables|SetClosestDistance (Math|Vector|VectorLength (- (Transformation|GetWorldLocation (Variables|/Game/RobertFunZone/Gun/VeryPlaceholderGun.VeryPlaceholderGun_C|GetStaticMesh _array_element)) (Transformation|GetActorLocation))))
      (LocalVariables|SetClosestTarget _array_element)))
  (return (Variables|/Game/RobertFunZone/Gun/VeryPlaceholderGun.VeryPlaceholderGun_C|GetStaticMesh (LocalVariables|GetClosestTarget))))