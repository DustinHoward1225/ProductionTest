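; BP_BulletWave is a temporary bullet actor that applies a looping vertical wave motion and destroys itself after WaitToDeleteWave seconds.
; Tick plays the WaveMovement timeline, which restarts itself on finish.
; Each update lerps Z from the current height toward 20 units above it, so offsets accumulate rather than following a fixed origin, while X and Y stay unchanged.
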(event Collision|EventActorBeginOverlap
  (params (OtherActor :type Actor%20Object%20Reference)))

(event EventTick
  (params (DeltaSeconds :type Float%20%28single-precision%29))
  (bind _returnvalue (Transformation|GetActorLocation))
  (bind _newtrack_0 (Timeline|WaveMovement Play)
    (:Update
      (Transformation|SetActorLocation (Math|Vector|MakeVector (.x _returnvalue) (.y _returnvalue) (Math|Float|Lerp (.z _returnvalue) (+ (.z _returnvalue) 2e+01) _newtrack_0)) false false))
    (:Finished
      (Timeline|WaveMovement PlayFromStart))))

(event EventBeginPlay
  (Utilities|FlowControl|Delay (Variables|Default|GetWaitToDeleteWave))
  (Actor|DestroyActor))

(fn ConstructionScript)