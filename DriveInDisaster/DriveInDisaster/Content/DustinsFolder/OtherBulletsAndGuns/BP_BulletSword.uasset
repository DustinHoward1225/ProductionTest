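; BP_BulletSword is a sword actor that can be picked up and dropped.
; Pickup turns off physics on the Swordbox component and attaches the root to the given component, keeping its world transform.
; Drop re-enables physics and detaches the actor in place.
; Unconnected leftover pawn code for spawning and destroying a SwordBullet never runs.
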(event EventBeginPlay)

(event EventDrop
  (Physics|SetSimulatePhysics (Variables|Default|Getswordbox) true)
  (Transformation|DetachFromActor "KeepWorld" "KeepWorld" "KeepWorld"))

(event EventPickup
  (params (AttachTo :type Scene%20Component%20Object%20Reference))
  (Physics|SetSimulatePhysics (Variables|Default|Getswordbox) false)
  (Transformation|AttachComponentToComponent (VehicleSound|GetRootComponent) AttachTo "None" "KeepWorld" "KeepWorld" "KeepWorld" true))

(fn ConstructionScript)