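; Laser bullet projectile actor that destroys itself three seconds after spawning unless its Test flag is set.
; A hit event destroys it, then adds a Niagara component and spawns a quiet sound using the Cube's position.
; Both hit events print debug strings, and the second does nothing else.
; Alternative LaserHit and BallHit sound calls are left unconnected.
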(event Custom|hit
  ;[1 1 1] G
  (Development|PrintString "nbv")
  (Actor|DestroyActor)
  (Variables|Default|SetHit%20Loc (Transformation|GetActorLocation))
  (bind _output_get (Variables|Default|SetHit%20Traqns (Transformation|GetWorldTransform (Variables|Default|GetCube))))
  (AddComponent|AddNiagaraComponent true (Math|Transform|MakeTransform (.location _output_get) (.rotation _output_get) "1,1,1"))
  (Audio|SpawnSoundatLocation 0 (Transformation|GetWorldLocation (Variables|Default|GetCube)) "0, 0, 0" 0.05 1.0 0.0 0 0))

(event Collision|EventHit
  (params (MyComp :type Primitive%20Component%20Object%20Reference) (Other :type Actor%20Object%20Reference) (OtherComp :type Primitive%20Component%20Object%20Reference) (bSelfMoved :type Boolean) (HitLocation :type Vector :default "0, 0, 0") (HitNormal :type Vector :default "0, 0, 0") (NormalImpulse :type Vector :default "0, 0, 0") (Hit :type Hit%20Result%20Structure%20%28by%20ref%29))
  ;[1 1 1] G
  (Development|PrintString "123123"))

(event EventBeginPlay
  ;[1 1 1] After 3 seconds destroys bullet
  (if (not (Variables|Default|Gettest))
    (Utilities|FlowControl|Delay 3.0)
    (Actor|DestroyActor)))

(fn ConstructionScript)