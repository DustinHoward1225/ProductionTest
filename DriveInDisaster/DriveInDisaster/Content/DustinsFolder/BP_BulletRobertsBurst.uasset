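; BP_BulletRobertsBurst is a bullet actor that despawns on impact or after a short airtime.
; BeginPlay runs a fixed delay, then destroys the actor if it is still flying.
; On Hit, it adds a Niagara component at the actor's transform, spawns an attenuated BallHit sound and destroys itself immediately.
; Despite the graph comment mentioning a physics impulse, the hit logic applies none.
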(event Collision|EventHit
  (params (MyComp :type Primitive%20Component%20Object%20Reference) (Other :type Actor%20Object%20Reference) (OtherComp :type Primitive%20Component%20Object%20Reference) (bSelfMoved :type Boolean) (HitLocation :type Vector :default "0, 0, 0") (HitNormal :type Vector :default "0, 0, 0") (NormalImpulse :type Vector :default "0, 0, 0") (Hit :type Hit%20Result%20Structure%20%28by%20ref%29))
  ;[1 1 1] physics impluse to hit object
  (Variables|Default|SetHitLoc (Transformation|GetActorLocation))
  (bind _output_get (Variables|Default|SetHitTraqns (Transformation|GetActorTransform)))
  (AddComponent|AddNiagaraComponent true _output_get)
  (Audio|SpawnSoundAttached "/Game/RobertFunZone/Audio/BallHit.BallHit" 0 "None" (Transformation|GetWorldLocation (Variables|Default|GetStaticMesh)) "0, 0, 0" "SnapToTarget" false 1.0 1.0 0.0 "/Game/RobertFunZone/Audio/Placeholder_Alien.Placeholder_Alien" 0)
  (Actor|DestroyActor))

(event EventBeginPlay
  ;[1 1 1] Destroys bullet after 3 seconds of airtime
  (Utilities|FlowControl|Delay 3.0)
  (Actor|DestroyActor))

(fn ConstructionScript)